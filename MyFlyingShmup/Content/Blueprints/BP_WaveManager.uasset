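; Wave manager that spawns enemies in sequential waves from the WaveData array, each wave defining enemy class, count, path, duration and initial delay.
; StartNextWave sets a SpawnEnemy timer with an interval of wave duration divided by enemy count.
; SpawnEnemy spawns an enemy at its path actor and starts it moving, or advances to the next wave when none remain.
; EndWaveSequence and EndCurrentWave are empty stubs.
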(event `StartWaveSequence`
  (set `self.CurrentWaveIndex` 0)
  (`self.StartNextWave`))

(event `EndWaveSequence`)

(event `StartNextWave`
  (bind (_output_name _output_id _output_numberofenemies _output_duration _output_initialdelay _output_enemyclass _output_enemypath) (break `/Game/Blueprints/S_Wave` (`|GetArrayItem` (`self.WaveData`) (`self.CurrentWaveIndex`))))
  (if (`KismetArrayLibrary.Array_IsValidIndex` (`self.WaveData`) (`self.CurrentWaveIndex`))
    (set `self.EnemiesRemainingInCurrentWave` _output_numberofenemies)
    (bind _returnvalue (`KismetSystemLibrary.K2_SetTimerDelegate` (delegate `SpawnEnemy`) (`KismetMathLibrary.SafeDivide` _output_duration (`KismetMathLibrary.Conv_IntToDouble` _output_numberofenemies)) false false _output_initialdelay))
    (set `self.WaveTimer` _returnvalue)))

(event `EndCurrentWave`)

(event `SpawnEnemy`
  (bind (_output_name _output_id _output_numberofenemies _output_duration _output_initialdelay _output_enemyclass _output_enemypath) (break `/Game/Blueprints/S_Wave` (`|GetArrayItem` (`self.WaveData`) (`self.CurrentWaveIndex`))))
  (if (> (`self.EnemiesRemainingInCurrentWave`) 0)
    (bind _returnvalue (`|SpawnActorFromClass` _output_enemyclass (`KismetMathLibrary.MakeTransform` (`self.K2_GetActorLocation` _output_enemypath)) "Undefined" "MultiplyWithRoot" null 0.0 _output_enemypath null))
    (`/Game/Blueprints/BP_BaseEnemy.StartMovingAlongPath` _returnvalue)
    (`/Engine/EditorBlueprintResources/StandardMacros.DecrementInt` (`self.EnemiesRemainingInCurrentWave`))
    (else
      (`KismetSystemLibrary.K2_PauseTimerHandle` (`self.WaveTimer`))
      (`/Engine/EditorBlueprintResources/StandardMacros.IncrementInt` (`self.CurrentWaveIndex`)
        (:`  `
          (`self.StartNextWave`))))))

(fn `UserConstructionScript`)