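; BP_EnemySpawner spawns random enemies and assigns each one a path to use.
; On BeginPlay it caches every BP_EnemyPath actor in the level.
; StartTimer, which is not called within this graph, starts a looping timer that spawns a random class from AllEnemies at a fixed location.
; Each spawned BP_BaseEnemy receives a random cached path.
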(event `self.ReceiveBeginPlay`
  (`self.GetAllPaths`))

(event `GetAllPaths`
  (bind _outactors (`GameplayStatics.GetAllActorsOfClass` "/Game/Blueprints/BP_EnemyPath.BP_EnemyPath_C"))
  (set `self.All Paths` _outactors))

(event `StartTimer`
  (`KismetSystemLibrary.K2_SetTimerDelegate` (delegate `SpawnEvent`) 1.0 true))

(event `SpawnEvent`
  (bind _returnvalue (`|SpawnActorFromClass` (`KismetArrayLibrary.Array_Random` (`self.All Enemies`)) (`KismetMathLibrary.MakeTransform` (10000.0 0.0 0.0)) "AlwaysSpawn" "MultiplyWithRoot" null null))
  (bind _asbp_base_enemy (cast `/Game/Blueprints/BP_BaseEnemy` _returnvalue))
  (set `/Game/Blueprints/BP_BaseEnemy.Path` (`KismetArrayLibrary.Array_Random` (`self.All Paths`)) _asbp_base_enemy))

(fn `UserConstructionScript`)