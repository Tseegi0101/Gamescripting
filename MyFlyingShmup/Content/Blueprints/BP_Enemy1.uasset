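; BP_Enemy1 is an enemy actor that gets a random sphere colour on BeginPlay through a dynamic material instance.
; It spawns a BP_EnemyBullet at its own transform every three seconds through a looping Delay.
; On overlap it subtracts the other actor's AC_Properties Damage from Health.
; At zero Health it adds to the WBP_Score widget, spawns a Niagara effect and destroys itself.
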(event `self.ReceiveBeginPlay`
  (bind (_returnvalue_location _returnvalue_rotation) (`KismetMathLibrary.BreakTransform` (`self.GetTransform`)))
  ; Random float colour changes
  (`|ExecutionSequence`
    (:`then_0`
      (bind _returnvalue (`KismetMaterialLibrary.CreateDynamicMaterialInstance` "/Game/Materials/MI_ColourLight.MI_ColourLight"))
      (`PrimitiveComponent.SetMaterial` (`self.Sphere_0`) 0 _returnvalue)
      (`MaterialInstanceDynamic.SetVectorParameterValue` _returnvalue "BaseColour" (`KismetMathLibrary.MakeColor` (`KismetMathLibrary.RandomFloat`) (`KismetMathLibrary.RandomFloat`) (`KismetMathLibrary.RandomFloat`))))
    (:`then_1`
      ; Comment
      (`|SpawnActorFromClass` "/Game/Blueprints/BP_EnemyBullet.BP_EnemyBullet_C" (`KismetMathLibrary.MakeTransform` _returnvalue_location _returnvalue_rotation) "Undefined" "MultiplyWithRoot" null null :!label _label)
      (`KismetSystemLibrary.Delay` 3.0)
      (goto _label))))

(event `self.ReceiveActorBeginOverlap`
  (params (OtherActor :type "Actor Object Reference"))
  ; Hit by Attack
  (`parent.ReceiveActorBeginOverlap` null)
  (bind _output_get (set `self.Health` (- (`self.Health`) (`/Game/Blueprints/AC_Properties.Damage` (`self.GetComponentByClass` OtherActor "/Game/Blueprints/AC_Properties.AC_Properties_C")))))
  (if (<= _output_get 0.0)
    ;;[1 0.03125 0.03125 0.5] Comment
    (bind _foundwidgets (`WidgetBlueprintLibrary.GetAllWidgetsOfClass` "/Game/Ui/WBP_Score.WBP_Score_C" false))
    (`/Game/Ui/WBP_Score.AddToScore` (`|GetArrayItem` _foundwidgets) 100)
    ; Collusion Effect
    (bind _returnvalue (`|SpawnActorFromClass` "/Script/Niagara.NiagaraActor" (`self.GetTransform`) "AlwaysSpawn" "MultiplyWithRoot" null null))
    (`NiagaraComponent.SetAsset` (`NiagaraActor.NiagaraComponent` _returnvalue) "/Game/Basic_VFX/Niagara/NS_Basic_2.NS_Basic_2" true)
    (`self.K2_DestroyActor`)))

(fn `UserConstructionScript`)