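; BP_BaseEnemy is a base enemy actor that travels along a spline path and reacts when something overlaps it.
; StartMovingAlongPath runs once, playing a slowed Timeline that samples the Path spline at constant velocity to set swept location and rotation, then destroys the actor when finished.
; Any overlap applies a flashing overlay material to all static mesh components and plays a 2D shot sound, with no damage or material reset.
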(event `StartMovingAlongPath`
  (bind _spline (`/Game/Blueprints/BP_EnemyPath.Spline` (`self.Path`)))
  (`/Engine/EditorBlueprintResources/StandardMacros.DoOnce` false
    (:`Completed`
      (`TimelineComponent.SetPlayRate` (`self.Timeline`) 0.2)
      (bind (_direction _newtrack_0) (`Timeline|Timeline`)
        (:`Update`
          (`self.K2_SetActorTransform` (`KismetMathLibrary.MakeTransform` (`SplineComponent.GetLocationAtTime` _spline _newtrack_0 "World" true) (`SplineComponent.GetRotationAtTime` _spline _newtrack_0 "World" true)) true))
        (:`Finished`
          (`self.K2_DestroyActor`))))))

(event `self.ReceiveActorBeginOverlap`
  (params (OtherActor :type "Actor Object Reference"))
  (for _array_element (`self.K2_GetComponentsByClass` "/Script/Engine.StaticMeshComponent")
    (`MeshComponent.SetOverlayMaterial` _array_element "/Game/Materials/MI_FlashingEnemy_Material.MI_FlashingEnemy_Material"))
  (`GameplayStatics.PlaySound2D` "/Game/Sci-Fi_Shots_Pack2_Game_Of_Weapons/Wave/SciFi_Shot_P2__100_.SciFi_Shot_P2__100_" 1.0 1.0 0.0 null null))

(fn `UserConstructionScript`)