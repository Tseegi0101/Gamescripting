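; BP_Enemy2 is an enemy actor that fires bullets on a timer and can be destroyed by contact.
; From BeginPlay, a looping Delay spawns a BP_EnemyBullet at the enemy's location and rotation immediately, then every four seconds.
; Any actor overlap calls the parent handler, then subtracts a fixed amount from Health without filtering the other actor, destroying the enemy at zero or below.
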(event `self.ReceiveBeginPlay`
  (bind (_returnvalue_location _returnvalue_rotation) (`KismetMathLibrary.BreakTransform` (`self.GetTransform`)))
  (`|SpawnActorFromClass` "/Game/Blueprints/BP_EnemyBullet.BP_EnemyBullet_C" (`KismetMathLibrary.MakeTransform` _returnvalue_location _returnvalue_rotation) "Undefined" "MultiplyWithRoot" null null :!label _label)
  (`KismetSystemLibrary.Delay` 4.0)
  (goto _label))

(event `self.ReceiveActorBeginOverlap`
  (params (OtherActor :type "Actor Object Reference"))
  (`parent.ReceiveActorBeginOverlap` null)
  (bind _output_get (set `self.Health` (- (`self.Health`) 100.0)))
  (if (<= _output_get 0.0)
    (`self.K2_DestroyActor`)))

(fn `UserConstructionScript`)