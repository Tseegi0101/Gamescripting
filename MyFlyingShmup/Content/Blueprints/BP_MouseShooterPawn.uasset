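; BP_MouseShooterPawn is a mouse-controlled pawn that moves toward the cursor and fires bullets.
; On possession it adds the mouse Enhanced Input mapping context and shows a crosshair cursor.
; The move action deprojects the cursor into a world trace, faces the hit point in XY and drives FloatingPawnMovement forward, setting max speed to the 2D distance to that point.
; The shoot action spawns BP_Bullet at the pawn's transform.
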(event `self.ReceivePossessed`
  (params (NewController :type "Controller Object Reference"))
  (bind _as_player_controller (`self.As Player Controller`))
  (bind _asplayer_controller (cast `PlayerController` NewController))
  (set `self.As Player Controller` _asplayer_controller)
  (message `EnhancedInputSubsystemInterface.AddMappingContext` (pcsubsystem `EnhancedInputLocalPlayerSubsystem` _asplayer_controller) "/Game/Inputs/IMC_MouseControls.IMC_MouseControls" 0 (struct))
  (set `PlayerController.bShowMouseCursor` true _as_player_controller)
  (set `PlayerController.CurrentMouseCursor` "Crosshairs" _as_player_controller))

(event `EnhancedInput|/Game/Inputs/IA_MoveWithMouse`
  (params (ActionValue :type Boolean) (ElapsedSeconds :type "Float (double-precision)") (TriggeredSeconds :type "Float (double-precision)") (InputAction :type "InputAction Object Reference" :default "/Game/Inputs/IA_MoveWithMouse.IA_MoveWithMouse"))
  (bind (_returnvalue_x _returnvalue_y) (`KismetMathLibrary.BreakVector` (`self.K2_GetActorLocation`)))
  (:`Triggered`
    (bind _returnvalue (`WidgetLayoutLibrary.GetMousePositionOnViewport`))
    (bind (_worldposition _worlddirection) (`GameplayStatics.DeprojectScreenToWorld` (`self.As Player Controller`) (* _returnvalue (`WidgetLayoutLibrary.GetViewportScale`))))
    (bind _outhit (`KismetSystemLibrary.LineTraceSingle` :`Start` _worldposition :`End` (+ _worldposition (* _worlddirection 5000.0) (0.0 0.0 0.0)) :`TraceChannel` "TraceTypeQuery1" :`DrawDebugType` "ForOneFrame"))
    (`self.K2_SetActorRotation` (`KismetMathLibrary.FindLookAtRotation` (`KismetMathLibrary.MakeVector` _returnvalue_x _returnvalue_y) (`KismetMathLibrary.MakeVector` (.x (`.Location` (`GameplayStatics.BreakHitResult` _outhit))) (.y (`.Location` (`GameplayStatics.BreakHitResult` _outhit))))))
    (`PawnMovementComponent.AddInputVector` (`self.FloatingPawnMovement`) (`self.GetActorForwardVector`) false)
    (set `FloatingPawnMovement.MaxSpeed` (`KismetMathLibrary.Distance2D` (`KismetMathLibrary.MakeVector2D` _returnvalue_x _returnvalue_y) (`KismetMathLibrary.MakeVector2D` (.x (`.Location` (`GameplayStatics.BreakHitResult` _outhit))) (.y (`.Location` (`GameplayStatics.BreakHitResult` _outhit))))) (`self.FloatingPawnMovement`))))

(event `EnhancedInput|/Game/Inputs/IA_ShootWithMouse`
  (params (ActionValue :type Boolean) (ElapsedSeconds :type "Float (double-precision)") (TriggeredSeconds :type "Float (double-precision)") (InputAction :type "InputAction Object Reference" :default "/Game/Inputs/IA_ShootWithMouse.IA_ShootWithMouse"))
  (:`Triggered`
    (`|SpawnActorFromClass` "/Game/Blueprints/BP_Bullet.BP_Bullet_C" (`self.GetTransform`) "Undefined" "MultiplyWithRoot" null null)))

(fn `UserConstructionScript`)