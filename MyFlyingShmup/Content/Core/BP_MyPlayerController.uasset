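; Player controller that sets the game's camera view and handles pausing and unpausing.
; On BeginPlay it blends the view to a CameraActor found in the level, and on possess it adds the global Enhanced Input mapping context.
; The pause action shows the BP_HUD pause menu with UI-only input and a cursor.
; UnpauseGame restores game-only input and hides the cursor, but leaves menu visibility untouched.
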(event `self.ReceiveBeginPlay`
  (bind _returnvalue (`GameplayStatics.GetActorOfClass` "/Script/Engine.CameraActor"))
  (`self.SetViewTargetWithBlend` _returnvalue))

(event `self.ReceivePossess`
  (params (PossessedPawn :type "Pawn Object Reference"))
  (bind _asplayer_controller (cast `PlayerController` (`Pawn.GetController` PossessedPawn)))
  (message `EnhancedInputSubsystemInterface.AddMappingContext` (pcsubsystem `EnhancedInputLocalPlayerSubsystem` _asplayer_controller) "/Game/Inputs/IMC_GlobalInputs.IMC_GlobalInputs" 0 (struct)))

(event `EnhancedInput|/Game/Inputs/IA_PauseGame`
  (params (ActionValue :type Boolean) (ElapsedSeconds :type "Float (double-precision)") (TriggeredSeconds :type "Float (double-precision)") (InputAction :type "InputAction Object Reference" :default "/Game/Inputs/IA_PauseGame.IA_PauseGame"))
  (:`Triggered`
    (bind _asbp_hud (cast `/Game/Core/BP_HUD` (`self.GetHUD`)))
    (bind _pausemenu (`/Game/Core/BP_HUD.PauseMenu` _asbp_hud))
    (set `Widget.Visibility` "Visible" _pausemenu)
    (`GameplayStatics.SetGamePaused` true)
    (`WidgetBlueprintLibrary.SetInputMode_UIOnlyEx` self _pausemenu "DoNotLock" true)
    (set `self.bShowMouseCursor` true))
  (:`Started`
    (if (not (`GameplayStatics.IsGamePaused`))
      _)))

(event `UnpauseGame`
  (`GameplayStatics.SetGamePaused` false)
  (`WidgetBlueprintLibrary.SetInputMode_GameOnly` self true)
  (set `self.bShowMouseCursor` false))

(fn `UserConstructionScript`)